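; BP_PathNode is a placeable path node that links to a next node to form a chain, with no active runtime logic.
; Its construction script registers itself as NextNode's PreviousNode and adds a straight two-point spline between the two locations.
; It also adds colored arrows facing the next and previous nodes, though the previous arrow appears only when a next node is set.
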(event EventBeginPlay)

(event Collision|EventActorBeginOverlap
  (params (OtherActor :type Actor%20Object%20Reference)))

(event EventTick
  (params (DeltaSeconds :type Float%20%28single-precision%29)))

(fn ConstructionScript
  (bind _self self)
  (bind _nextnode (Variables|Default|GetNextNode))
  (bind _returnvalue (Transformation|GetActorLocation _self))
  (bind _returnvalue_2 (Transformation|GetActorLocation _nextnode))
  (Utilities|IsValid (Variables|Default|GetNextNode)
    (:Is%20Valid
      (Utilities|FlowControl|Sequence
        (:then_0
          (Variables|BP_PathNode_C|SetPreviousNode (Variables|Default|GetNextNode) self))
        (:then_1
          (bind _returnvalue_3 (AddComponent|AddSplineComponent false))
          (Spline|SetSplinePoints _returnvalue_3 (Utilities|Array|MakeArray _returnvalue _returnvalue_2) "World" true))
        (:then_2
          (bind _returnvalue_4 (AddComponent|AddArrowComponent false (Math|Transform|MakeTransform "0, 0, 0" (Math|Rotator|FindLookatRotation _returnvalue _returnvalue_2) "1.000000,1.000000,1.000000")))
          (Variables|/Script/Engine.ArrowComponent|SetArrowColor _returnvalue_4 (Variables|Default|GetNextNodeArrowColor)))
        (:then_3
          (Utilities|IsValid (Variables|Default|GetPreviousNode)
            (:Is%20Valid
              (bind _returnvalue_5 (AddComponent|AddArrowComponent false (Math|Transform|MakeTransform "0, 0, 0" (Math|Rotator|FindLookatRotation _returnvalue (Transformation|GetActorLocation (Variables|Default|GetPreviousNode))) "1.000000,1.000000,1.000000")))
              (Variables|/Script/Engine.ArrowComponent|SetArrowColor _returnvalue_5 (Variables|Default|GetPreviousNodeArrowColor)))))))))