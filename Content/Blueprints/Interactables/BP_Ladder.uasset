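; BP_Ladder is an interactable ladder that teleports the player instead of animating a climb.
; On interact, it moves player character 0 to its Scene component's world location, keeping the character's rotation.
; BeginPlay creates a dynamic instance of M_Ladder on the static mesh, and hover start and end toggle its EmissiveStrength as a highlight.
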(event EventBeginPlay
  (bind _returnvalue (Rendering|Material|CreateDynamicMaterialInstance (Variables|Default|GetStaticMesh) 0 "/Game/Materials/Instances/M_Ladder.M_Ladder" "None" :!class /Script/Engine.PrimitiveComponent))
  (Variables|Default|SetMaterialInstance _returnvalue))

(event EventOnHoverStart
  (Rendering|Material|SetScalarParameterValue (Variables|Default|GetMaterialInstance) (Utilities|Name|MakeLiteralName "EmissiveStrength") 2.0 :!class /Script/Engine.MaterialInstanceDynamic))

(event EventOnInteract
  (bind _returnvalue (Game|GetPlayerCharacter 0))
  (Transformation|Teleport _returnvalue (Transformation|GetWorldLocation (Variables|Default|GetScene)) (Transformation|GetActorRotation _returnvalue)))

(event EventOnHoverEnd
  (Rendering|Material|SetScalarParameterValue (Variables|Default|GetMaterialInstance) (Utilities|Name|MakeLiteralName "EmissiveStrength") 0.0 :!class /Script/Engine.MaterialInstanceDynamic))

(fn ConstructionScript)