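; BP_Lectern is an interactable lectern with an open book that removes a linked Barrier actor when interacted with.
; On BeginPlay it creates a dynamic instance of M_Book on the BookOpened component.
; Hover start and end events drive that material's EmissiveStrength to make the book glow as a highlight, with a debug print on hover.
; Interacting destroys the referenced Barrier.
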(event EventBeginPlay
  (bind _returnvalue (Rendering|Material|CreateDynamicMaterialInstance (Variables|Default|GetBook_opened) 0 "/Game/Materials/Instances/M_Book.M_Book" "None" :!class /Script/Engine.PrimitiveComponent))
  (Variables|Default|SetMaterialInstance _returnvalue))

(event EventOnHoverEnd
  (Rendering|Material|SetScalarParameterValue (Variables|Default|GetMaterialInstance) (Utilities|Name|MakeLiteralName "EmissiveStrength") 0.0 :!class /Script/Engine.MaterialInstanceDynamic))

(event EventOnHoverStart
  (Development|PrintString "Hovered!" true true "(R=0.000000,G=0.660000,B=1.000000,A=1.000000)" 2.0 "hover")
  (Rendering|Material|SetScalarParameterValue (Variables|Default|GetMaterialInstance) (Utilities|Name|MakeLiteralName "EmissiveStrength") 2.0 :!class /Script/Engine.MaterialInstanceDynamic))

(event EventOnInteract
  (Actor|DestroyActor (Variables|Default|GetBarrier)))

(fn ConstructionScript)