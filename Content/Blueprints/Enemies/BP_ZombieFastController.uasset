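; AI controller for the fast zombie enemy that runs a behavior tree and feeds it perception data through the blackboard.
; On BeginPlay it starts the tree and stores the pawn's spawn position as StartLocation.
; Each perception update writes whether the stimulus was sensed to HasDetectedPlayer? and its position to TargetLocation, without filtering by the sensed actor.
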(event OnTargetPerceptionUpdated(AIPerception)
  (params (Actor :type Actor%20Object%20Reference) (Stimulus :type AI%20Stimulus%20Structure))
  (bind (_age _expirationage _strength _stimuluslocation _receiverlocation _tag _bsuccessfullysensed) (Utilities|Struct|BreakAIStimulus Stimulus))
  (Utilities|FlowControl|Sequence
    (:then_0
      (AI|Components|Blackboard|SetValueasBool (AI|GetBlackboard 0) (Utilities|Name|MakeLiteralName "HasDetectedPlayer?") _bsuccessfullysensed))
    (:then_1
      (AI|Components|Blackboard|SetValueasVector (AI|GetBlackboard 0) (Utilities|Name|MakeLiteralName "TargetLocation") _stimuluslocation))))

(event EventBeginPlay
  (AI|RunBehaviorTree)
  (AI|Components|Blackboard|SetValueasVector (AI|GetBlackboard 0) (Utilities|Name|MakeLiteralName "StartLocation") (Transformation|GetActorLocation (Pawn|GetControlledPawn))))

(fn ConstructionScript)