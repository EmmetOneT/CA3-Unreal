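; AI controller for the slow zombie enemy, running the SlowZombie_BT behavior tree.
; On BeginPlay it starts the tree and stores the controlled pawn's location in the blackboard as StartLocation.
; AI perception updates write the stimulus location to TargetLocation, with a switch on the stimulus tag in that event.
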(event OnTargetPerceptionUpdated(AIPerception)
  (params (Actor :type Actor%20Object%20Reference) (Stimulus :type AI%20Stimulus%20Structure))
  (bind (_age _expirationage _strength _stimuluslocation _receiverlocation _tag) (Utilities|Struct|BreakAIStimulus Stimulus))
  (switch name _tag
    (:throwable
      (AI|Components|Blackboard|SetValueasVector (AI|GetBlackboard 0) (Utilities|Name|MakeLiteralName "TargetLocation") _stimuluslocation))))

(event EventBeginPlay
  (AI|RunBehaviorTree "/Game/AI/SlowZombie_BT.SlowZombie_BT")
  (AI|Components|Blackboard|SetValueasVector (AI|GetBlackboard 0) (Utilities|Name|MakeLiteralName "StartLocation") (Transformation|GetActorLocation (Pawn|GetControlledPawn))))

(fn ConstructionScript)